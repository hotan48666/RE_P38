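; P38__PawnBP is a player-controlled aircraft pawn that constantly flies forward and fires rockets.
; Roll and Pitch axes apply clamped, delta-time-scaled local rotation, steering the forward movement input added every tick.
; Tick also spins both propeller meshes through the shared PropellerRotation function.
; Fire spawns Rocket_BP at the Body transform, while holding Boot raises the FloatingPawnMovement max speed as a boost and releasing it lowers it.
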(event `self.ReceiveBeginPlay`
  ;[0 1 0.3672] 입력을 받을수 있도록 변경
  (`self.EnableInput` (`GameplayStatics.GetPlayerController` 0)))

(event `InputAxis|Roll`
  (params (AxisValue :type "Float (single-precision)"))
  (`self.K2_AddActorLocalRotation` (`KismetMathLibrary.MakeRotator` (* (`KismetMathLibrary.FClamp` AxisValue -1.0) (`self.RotationSpeed`) (`GameplayStatics.GetWorldDeltaSeconds`)))))

(event `InputAxis|Pitch`
  (params (AxisValue :type "Float (single-precision)"))
  (`self.K2_AddActorLocalRotation` (`KismetMathLibrary.MakeRotator` 0.0 (* (`KismetMathLibrary.FClamp` AxisValue -1.0) (`self.RotationSpeed`) (`GameplayStatics.GetWorldDeltaSeconds`)))))

(event `InputAction|Fire`
  (params (Key :type "Key Structure"))
  (:`Pressed`
    (`|SpawnActorFromClass` "/Game/Blueprints/Rocket_BP.Rocket_BP_C" (`SceneComponent.K2_GetComponentToWorld` (`self.Body`)) "Undefined" "OverrideRootScale" null null)))

(event `self.ReceiveTick`
  (params (DeltaSeconds :type "Float (single-precision)"))
  ;[1 0.7969 0] 오른쪽 회전
  (`self.PropellerRotation` (`self.PropellerR`))
  ;[0 0.5781 1] 왼쪽 회전
  (`self.PropellerRotation` (`self.PropellerL`))
  (`self.AddMovementInput` (`self.GetActorForwardVector`)))

(event `InputAction|Boot`
  (params (Key :type "Key Structure"))
  (:`Pressed`
    (bind _output_get (set `self.MoveSpeed` 400.0))
    (set `FloatingPawnMovement.MaxSpeed` _output_get (`self.FloatingPawnMovement`)))
  (:`Released`
    (bind _output_get_2 (set `self.MoveSpeed` 50.0))
    (set `FloatingPawnMovement.MaxSpeed` _output_get_2 (`self.FloatingPawnMovement`))))

(fn `PropellerRotation`
  (params (Mesh :type "SceneComponent Object Reference"))
  (`SceneComponent.K2_AddLocalRotation` Mesh (`KismetMathLibrary.MakeRotator` (* (`self.PropellerSpeed`) (`GameplayStatics.GetWorldDeltaSeconds`))) false false))

(fn `UserConstructionScript`)