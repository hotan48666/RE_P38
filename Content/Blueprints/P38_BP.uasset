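; P38_BP is a P-38 aircraft actor that spins its two propellers and moves along the world X axis.
; Each Tick calls PropellerRotation to add local roll to both propeller meshes, then adds a world-space X offset to Body.
; Both steps add delta seconds to their speed values rather than multiplying, so motion depends on frame rate.
; BeginPlay enables input for player 0, though the graph handles no input events.
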(event `self.ReceiveBeginPlay`
  (`self.EnableInput` (`GameplayStatics.GetPlayerController` 0)))

(event `self.ReceiveTick`
  (params (DeltaSeconds :type "Float (single-precision)"))
  (`self.PropellerRotation` (`self.PropellerR`))
  (`self.PropellerRotation` (`self.PropellerL`))
  (`SceneComponent.K2_AddWorldTransform` (`self.Body`) (`KismetMathLibrary.MakeTransform` (`KismetMathLibrary.MakeVector` (+ (`self.MoveSpeed`) (`GameplayStatics.GetWorldDeltaSeconds`)))) false false))

(fn `PropellerRotation`
  (params (Mesh :type "SceneComponent Object Reference"))
  (`SceneComponent.K2_AddLocalRotation` Mesh (`KismetMathLibrary.MakeRotator` (+ (`self.Propeller`) (`GameplayStatics.GetWorldDeltaSeconds`))) false false))

(fn `UserConstructionScript`)